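; BP_AutoFense is a procedural fence Blueprint that places repeated static meshes in its construction script.
; The segment count comes from the length of FenseEnd, with one mesh every 20 units along UnitVector, rotated to face that direction.
; Each segment gets a tiny random Z scale variation.
; The node that derives UnitVector from FenseEnd is never executed, so placement uses the variable's stored value.
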(fn `UserConstructionScript`
  (bind _unitvector (`self.UnitVector`))
  (for _index (range 1 (+ (`KismetMathLibrary.FTrunc` (/ (`KismetMathLibrary.VSize` (`self.FenseEnd`)) 20.0)) 1))
    (`AddComponent|NODE_AddStaticMeshComponent-0` :`RelativeTransform` (`KismetMathLibrary.MakeTransform` (* _index 20 _unitvector) (`KismetMathLibrary.Conv_VectorToRotator` _unitvector) (`KismetMathLibrary.MakeVector` 1.0 1.0 (`KismetMathLibrary.RandomFloatInRange` 0.999 1.001))))))