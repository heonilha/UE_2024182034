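; BP_GoldTrophy is a floating trophy actor that explodes and disappears when something overlaps it.
; It stores its start location on BeginPlay, then bobs vertically each Tick using a time-based sine wave scaled by Frequency and Amplitude.
; Any overlap with its Capsule spawns an explosion particle at the actor's location and destroys it, with no check on the other actor and no scoring.
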(event `self.Capsule.OnComponentBeginOverlap`
  (params (OverlappedComponent :type "PrimitiveComponent Object Reference") (OtherActor :type "Actor Object Reference") (OtherComp :type "PrimitiveComponent Object Reference") (OtherBodyIndex :type Integer) (bFromSweep :type Boolean) (SweepResult :type "HitResult Structure (by ref)"))
  (`GameplayStatics.SpawnEmitterAtLocation` "/Game/StarterContent/Particles/P_Explosion.P_Explosion" (`self.K2_GetActorLocation`))
  (`self.K2_DestroyActor`))

(event `self.ReceiveBeginPlay`
  (set `self.StartLocation` (`self.K2_GetActorLocation`)))

(event `self.ReceiveTick`
  (params (DeltaSeconds :type "Float (single-precision)"))
  (`self.K2_SetActorLocation` (+ (`self.StartLocation`) (`KismetMathLibrary.MakeVector` 0.0 0.0 (* (`KismetMathLibrary.Sin` (* (`GameplayStatics.GetTimeSeconds`) (`KismetMathLibrary.MultiplyByPi` 2.0) (`self.Frequency`))) (`self.Amplitude`))))))

(fn `UserConstructionScript`)